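; Player stats component that links the player's stats to the bars on the main HUD widget.
; InitializeManager stores the player reference and sets up stats, and OnStatsSetUp then initializes a bar for each stat key with its value.
; UpdateStat pushes a stat's current value to its bar, with GetBarForStat mapping Shield, Health and Objective to their widget bars.
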(event Custom|InitializeManager
  (params (Player :type Top%20Down%20Character%20Object%20Reference))
  (Variables|Default|SetPlayerRef Player)
  (CallFunction|SetUpStats))

(event EventOnStatsSetUp
  (bind _keys (Utilities|Map|Keys (Variables|Default|GetStats)))
  (for _array_element _keys
    (Default|InitializeBar (CallFunction|GetBarforStat _array_element) (.StatValue (CallFunction|GetStat _array_element)))))

(event EventUpdateStat
  (params (Stat :type E_Stats%20Enum :default "NewEnumerator0"))
  (Default|UpdateStat (CallFunction|GetBarforStat Stat) (.CurrentValue (CallFunction|GetStat Stat))))

(fn GetBarforStat
  (params (Stat :type E_Stats%20Enum :default "NewEnumerator0"))
  (bind _playerref (Variables|Default|GetPlayerRef))
  (bind _mainwidget (Variables|/Game/TopDownBP/Blueprints/TopDownCharacter.TopDownCharacter_C|GetMainWidget _playerref))
  (return (Utilities|Select :Index Stat :NewEnumerator0 0 :NewEnumerator1 (Variables|/Game/Building/Widgets/W_Main.W_Main_C|GetShieldBar _mainwidget) :NewEnumerator2 (Variables|/Game/Building/Widgets/W_Main.W_Main_C|GetHealthBar _mainwidget) :NewEnumerator3 (Variables|/Game/Building/Widgets/W_Main.W_Main_C|GetObjectiveHealthBar _mainwidget))))