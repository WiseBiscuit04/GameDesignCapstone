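; BalistaeShot is a projectile actor, apparently the bolt fired by a ballista buildable.
; On BeginPlay it launches itself by adding a force along its forward vector to its BallistaeShot component.
; When it hits an actor whose class is exactly BasicEnemy, it applies damage and destroys itself; any other hit is ignored.
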(event EventBeginPlay
  (Physics|AddForce (Variables|Default|GetBallistae_Shot) (* (Transformation|GetActorForwardVector self) 2.5e+02) "None" false))

(event Collision|EventHit
  (params (MyComp :type Primitive%20Component%20Object%20Reference) (Other :type Actor%20Object%20Reference) (OtherComp :type Primitive%20Component%20Object%20Reference) (bSelfMoved :type Boolean) (HitLocation :type Vector :default "0, 0, 0") (HitNormal :type Vector :default "0, 0, 0") (NormalImpulse :type Vector :default "0, 0, 0") (Hit :type Hit%20Result%20Structure%20%28by%20ref%29))
  (if (== (Utilities|GetClass Other) "/Game/TopDownBP/Blueprints/AI/BasicEnemy.BasicEnemy_C")
    (Game|Damage|ApplyDamage Other 1.0 0 0)
    (Actor|DestroyActor)))

(fn ConstructionScript)