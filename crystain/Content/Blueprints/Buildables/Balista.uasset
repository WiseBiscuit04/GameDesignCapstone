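; Buildable ballista that automatically fires shots at an enemy standing in its forward line of sight.
; A looping timer started at BeginPlay runs a forward line trace on the Visibility channel, with persistent debug drawing and a printout of the hit actor's name.
; When the hit actor equals BasicEnemy, it spawns a BalistaeShot just in front of itself and pushes it forward with AddForce.
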(event Custom|Conditional%20Fire
  (bind _self self)
  (bind _self_2 self)
  (bind _returnvalue (Transformation|GetActorForwardVector _self))
  (bind _returnvalue_2 (Transformation|GetActorLocation _self_2))
  (bind _returnvalue_3 (* _returnvalue 2e+01))
  (bind _outhit (Collision|LineTraceByChannel _returnvalue_2 (+ _returnvalue_2 (* (Transformation|GetActorForwardVector _self_2) 5e+03)) "TraceTypeQuery1" false 0 "Persistent"))
  (Development|PrintString (Utilities|GetDisplayName (.HitActor (Collision|BreakHitResult _outhit))))
  (if (== (.HitActor (Collision|BreakHitResult _outhit)) "/Game/TopDownBP/Blueprints/AI/BasicEnemy.BasicEnemy")
    (bind _returnvalue_4 (Game|SpawnActorfromClass "/Game/Blueprints/Buildables/BalistaeShot.BalistaeShot_C" (Math|Conversions|ToTransform(Vector) (+ (Transformation|GetActorLocation _self) _returnvalue_3)) "Undefined" 0 0))
    (Physics|AddForce (Variables|/Game/Blueprints/Buildables/BalistaeShot.BalistaeShot_C|GetBallistae_Shot _returnvalue_4) _returnvalue_3 "None" false)))

(event EventBeginPlay
  (Utilities|Time|SetTimerbyEvent (delegate Custom|Conditional%20Fire) 1.0 true))

(fn ConstructionScript)