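; Enemy wave spawner that places BasicEnemy actors on a one-second looping timer and ends the level on victory.
; Each tick spawns one enemy, cycling through three spawn locations, while the live count is under the cap and the total quota remains.
; When all enemies have spawned and none remain, it shows the Victory widget and opens MainMenu after a five-second delay.
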(event Custom|Spawn%20Enemy
  (if (and (== (Variables|Default|GetCurrent%20Enemies) 0) (== (Variables|Default|GetTotal%20Enemies%20Spawned) (Variables|Default|GetTotal%20Enemies)))
    (bind _returnvalue (UserInterface|CreateWidget "/Game/UI/Victory.Victory_C"))
    (UserInterface|Viewport|AddtoViewport _returnvalue 0)
    (Utilities|FlowControl|Delay 5.0)
    (Game|OpenLevel(byName) "MainMenu")
    (elif (< (Variables|Default|GetCurrent%20Enemies) (Variables|Default|GetMax%20Spawned))
      (if (< (Variables|Default|GetTotal%20Enemies%20Spawned) (Variables|Default|GetTotal%20Enemies))
        (Game|SpawnActorfromClass "/Game/TopDownBP/Blueprints/AI/BasicEnemy.BasicEnemy_C" (Utilities|Array|Get(acopy) (Variables|Default|GetSpawn%20Locations) (Variables|Default|GetCurrent%20Location)) "AdjustIfPossibleButAlwaysSpawn" 0 0)
        (Math|Integer|IncrementInt (Variables|Default|GetCurrent%20Enemies)
          (:%20%20
            (Math|Integer|IncrementInt (Variables|Default|GetTotal%20Enemies%20Spawned)
              (:%20%20
                (if (== (Variables|Default|GetCurrent%20Location) 2)
                  (Variables|Default|SetCurrent%20Location 0)
                  (else
                    (Math|Integer|IncrementInt (Variables|Default|GetCurrent%20Location))))))))))))

(event EventBeginPlay
  (Utilities|Time|SetTimerbyEvent (delegate Custom|Spawn%20Enemy) 1.0 true))

(fn ConstructionScript)